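; Parkour elevator actor that shuttles continuously between its starting location and the location of a Target actor.
; On BeginPlay it caches both endpoints, sets the timeline play rate from Speed and starts the timeline.
; The timeline alpha lerps the actor's location without sweeping, and its Finished event flips playback direction for an endless ping-pong.
; Overlap and Tick events are empty, and a delayed-reverse branch is left unconnected.
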(event `self.ReceiveBeginPlay`
  (`TimelineComponent.SetPlayRate` (`self.Timeline_1`) (`self.Speed`))
  (set `self.InitialLocation` (`self.K2_GetActorLocation`))
  (set `self.Destination` (`self.K2_GetActorLocation` (`self.Target`)))
  (bind (_direction _newtrack_1) (`Timeline|Timeline_1` :!label _label)
    (:`Update`
      (`/Engine/EditorBlueprintResources/StandardMacros.IsValid` "Elevator"
        (:`Is Valid`
          (`self.K2_SetActorLocation` (`KismetMathLibrary.VLerp` (`self.InitialLocation`) (`self.Destination`) _newtrack_1)))))
    (:`Finished`
      (bind _output_get (set `self.DirectionMoving` _direction))
      (if (`|EnumEquality` _output_get "Forward")
        (goto _label :!via `Reverse`)
        (else
          (goto _label))))))

(event `self.ReceiveActorBeginOverlap`
  (params (OtherActor :type "Actor Object Reference")))

(event `self.ReceiveTick`
  (params (DeltaSeconds :type "Float (single-precision)")))

(fn `UserConstructionScript`)