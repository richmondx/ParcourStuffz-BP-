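; Elevator actor for the parcour assets that rises when another actor overlaps it and returns down once nothing overlaps it.
; Overlap sets an Elevating flag, switches a mesh material to emissive red after a short delay, then plays a timeline lerping world Z between fixed heights.
; While not elevating, Tick checks for overlapping actors and, if none, reverses the timeline after a delay.
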(event `self.ReceiveActorBeginOverlap`
  (params (OtherActor :type "Actor Object Reference"))
  (set `self.Elevating` true)
  (`KismetSystemLibrary.Delay` 0.4)
  (`PrimitiveComponent.SetMaterial` (`self.StaticMeshComponent`) 1 "/Game/Emissive_RED.Emissive_RED")
  (`KismetSystemLibrary.Delay` 0.6)
  (bind (_direction _newtrack_1) (`Timeline|Timeline_0` :!label _label)
    (:`Update`
      (`/Engine/EditorBlueprintResources/StandardMacros.IsValid` "OnOverlapElevator"
        (:`Is Valid`
          (`self.K2_SetActorLocation` (`KismetMathLibrary.MakeVector` (.x (`self.K2_GetActorLocation`)) (.y (`self.K2_GetActorLocation`)) (`KismetMathLibrary.Lerp` 1.0 500.0 _newtrack_1))))
        (:`Is Not Valid`
          (`KismetSystemLibrary.PrintText` "FUCK SOMETHING WENT WRONG!"))))
    (:`Finished`
      (set `self.Elevating` false))))

(event `self.ReceiveTick`
  (params (DeltaSeconds :type "Float (single-precision)"))
  (if (`self.Elevating`)
    _
    (elif (<= (`KismetArrayLibrary.Array_Length` (`self.GetOverlappingActors` null)) 0)
      (`KismetSystemLibrary.Delay` 2.0)
      (set `self.Elevating` true)
      (goto _label :!via `Reverse`))))

(fn `UserConstructionScript`)